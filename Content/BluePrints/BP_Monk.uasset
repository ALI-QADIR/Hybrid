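; BP_Monk is a monk character Blueprint that plays four melee attacks: punch, mid kick, jump kick and high kick.
; Each trigger event plays its PaperZD animation override in the shared AttackOverrideSlot of the animation component's AnimInstance.
; An IsAttacking flag is set when playback starts and cleared on completion or cancellation.
; The file contains no input binding, damage or hit detection logic.
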(event EventBeginPlay)

(event Collision|EventActorBeginOverlap
  (params (OtherActor :type Actor%20Object%20Reference)))

(event EventHighKickTriggered
  (|PlayAnimationOverridewithCallbacks (Variables|/Script/PaperZD.PaperZDAnimationComponent|GetAnimInstance (Variables|Default|GetAnimationComponent)) "/Game/BluePrints/AnimSequences/HighKick.HighKick" "AttackOverrideSlot" 1.0 0.0
    (:then
      (Class|Monk|SetIsAttacking true))
    (:OnCompleted
      (Class|Monk|SetIsAttacking false :!label _label))
    (:OnCancelled
      (goto _label))))

(event EventTick
  (params (DeltaSeconds :type Float%20%28single-precision%29)))

(event EventPunchTriggered
  (|PlayAnimationOverridewithCallbacks (Variables|/Script/PaperZD.PaperZDAnimationComponent|GetAnimInstance (Variables|Default|GetAnimationComponent)) "/Game/BluePrints/AnimSequences/Punch.Punch" "AttackOverrideSlot" 1.0 0.0
    (:then
      (Class|Monk|SetIsAttacking true))
    (:OnCompleted
      (Class|Monk|SetIsAttacking false :!label _label))
    (:OnCancelled
      (goto _label))))

(event EventKickTriggered
  (|PlayAnimationOverridewithCallbacks (Variables|/Script/PaperZD.PaperZDAnimationComponent|GetAnimInstance (Variables|Default|GetAnimationComponent)) "/Game/BluePrints/AnimSequences/MidKick.MidKick" "AttackOverrideSlot" 1.0 0.0
    (:then
      (Class|Monk|SetIsAttacking true))
    (:OnCompleted
      (Class|Monk|SetIsAttacking false :!label _label))
    (:OnCancelled
      (goto _label))))

(event EventJumpKickTriggered
  (|PlayAnimationOverridewithCallbacks (Variables|/Script/PaperZD.PaperZDAnimationComponent|GetAnimInstance (Variables|Default|GetAnimationComponent)) "/Game/BluePrints/AnimSequences/JumpKick.JumpKick" "AttackOverrideSlot" 1.0 0.0
    (:then
      (Class|Monk|SetIsAttacking true))
    (:OnCompleted
      (Class|Monk|SetIsAttacking false :!label _label))
    (:OnCancelled
      (goto _label))))

(fn ConstructionScript)